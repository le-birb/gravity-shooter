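; A shootable contraption switch that activates once when FirstPersonProjectile hits have worn its health down to zero.
; Each hit on its Box subtracts BulletDamage, and depletion swaps the SwitchStandIn material and fires EventActivated through a DoOnce.
; While health sits between zero and max, Tick regenerates it based on RegenTime, using TimeBuffer to carry fractional healing into the integer health value.
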(event `self.Box.OnComponentHit`
  (params (HitComponent :type "PrimitiveComponent Object Reference") (OtherActor :type "Actor Object Reference") (OtherComp :type "PrimitiveComponent Object Reference") (NormalImpulse :type "Vector Structure") (Hit :type "HitResult Structure (by ref)"))
  (cast `/Game/FirstPersonBP/Blueprints/FirstPersonProjectile` OtherActor)
  (bind _output_get (set `self.CurrentHealth` (- (`self.CurrentHealth`) (`self.BulletDamage`))))
  (if (<= _output_get 0)
    (`/Engine/EditorBlueprintResources/StandardMacros.DoOnce` false
      (:`Completed`
        (`PrimitiveComponent.SetMaterial` (`self.SwitchStandIn`) 0 "/Game/Geometry/Meshes/SwitchMaterial.SwitchMaterial")
        (`self.EventActivated`)))))

(event `self.ReceiveTick`
  (params (DeltaSeconds :type "Float (single-precision)"))
  (bind _currenthealth (`self.CurrentHealth`))
  (bind (_remainder _returnvalue) (`KismetMathLibrary.FMod` (+ (`self.TimeBuffer`) (/ DeltaSeconds (`self.RegenTime`))) 1.0))
  ;[1 1 1] Only proceed if 0 < health < max
  (if (> _currenthealth 0)
    (if (< _currenthealth (`self.MaxHealth`))
      (set `self.TimeBuffer` _remainder) ; Put remaining decimal back in buffer
      (set `self.CurrentHealth` (`KismetMathLibrary.Clamp` (+ _returnvalue (`self.CurrentHealth`)) 0 (`self.MaxHealth`))) ; Add integer part to health (clamp to max)
    )))

(fn `UserConstructionScript`
  (`parent.UserConstructionScript`))