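; SwitchTimerBP is a switch contraption that turns on momentarily when shot.
; A first-person projectile hitting its box swaps the stand-in mesh to the on material and calls the activated event.
; A short fixed timer then runs Deactivate, which restores the off material and calls the deactivated event.
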(event `self.Box.OnComponentHit`
  (params (HitComponent :type "PrimitiveComponent Object Reference") (OtherActor :type "Actor Object Reference") (OtherComp :type "PrimitiveComponent Object Reference") (NormalImpulse :type "Vector Structure") (Hit :type "HitResult Structure (by ref)"))
  (cast `/Game/FirstPersonBP/Blueprints/FirstPersonProjectile` OtherActor)
  (`PrimitiveComponent.SetMaterial` (`self.SwitchStandIn`) 0 "/Game/Geometry/Meshes/SwitchMaterial.SwitchMaterial")
  (`self.EventActivated`)
  (`KismetSystemLibrary.K2_SetTimer` null "deactivate" 0.1))

(fn `deactivate`
  (`PrimitiveComponent.SetMaterial` (`self.SwitchStandIn`) 0 "/Game/Geometry/Meshes/SwitchOffMaterial.SwitchOffMaterial")
  (`self.EventDeactivated`))

(fn `UserConstructionScript`
  (`parent.UserConstructionScript`))